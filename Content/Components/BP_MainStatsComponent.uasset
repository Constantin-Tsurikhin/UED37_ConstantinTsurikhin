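; Actor component holding an entity's core stats: HP, EP shields, walk speed, behavior and fraction.
; On BeginPlay it loads the CurrentName row from DT_AllStates to configure them, restoring saved HP/EP for the player outside a new game, otherwise filling to max.
; ReceiveDamage reduces only HP and flags death, while HealUp and ShieldUp restore values up to their maximums.
; Changes are broadcast through stats-updated, damage and death events.
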(event EventBeginPlay
  (Configuration|ConfigureStats))

(event EventTick
  (params (DeltaSeconds :type Float%20%28single-precision%29)))

(fn ConfigureStats
  (if (Utilities|Name|NotEqual(Name) (Variables|Default|GetCurrentName) "")
    (bind _returnvalue (Utilities|GetDataTableRow "/Game/Data/DT_AllStates.DT_AllStates" (Variables|Default|GetCurrentName))
      (:then
        (Variables|Default|SetMainStatsStructure _returnvalue)
        (Utilities|FlowControl|Sequence
          (:then_0
            (Configuration|ConfigureMovement))
          (:then_1
            (Configuration|ConfigureHealthandShields))
          (:then_2
            (Configuration|ConfigureBehaviorandFraction))))
      (:RowNotFound
        (Development|PrintString "Configure Stats Failed: Current name is not found in DT" false)))
    (else
      (Development|PrintString "Configure Stats Failed: Current name is invalid" false))))

(fn ReceiveDamage
  (params (InDamage :type Float%20%28single-precision%29) (InType :type ENUM_DamageType%20Enum :default "NewEnumerator0") (InCauser :type Actor%20Object%20Reference))
  (if (not (Variables|Default|GetIsDead))
    (Variables|Default|SetCurrentHP (- (Variables|Default|GetCurrentHP) (Math|Float|Truncate InDamage)))
    (if (> (Variables|Default|GetCurrentHP) 0)
      (Variables|Default|SetIsDead false)
      (else
        (Variables|Default|SetCurrentHP 0)
        (Variables|Default|SetIsDead true)))
    (Default|CallOnStatsUpdated (Variables|Default|GetCurrentHP) (Variables|Default|GetCurrentEP) (Variables|Default|GetIsDead) true)
    (if (Variables|Default|GetIsDead)
      (Default|CallOnDied)
      (else
        (Default|CallOnDamageReceived InDamage InType InCauser)))))

(fn HealUp
  (params (InToMaximum :type Boolean) (InAddHP :type Integer))
  (if InToMaximum
    (Variables|Default|SetCurrentHP (.MaxHP (Utilities|Struct|BreakSTRUCT_MainStates (Variables|Default|GetMainStatsStructure))))
    (else
      (Variables|Default|SetCurrentHP (Math|Integer|Min(Integer) (+ (Variables|Default|GetCurrentHP) InAddHP) (.MaxHP (Utilities|Struct|BreakSTRUCT_MainStates (Variables|Default|GetMainStatsStructure)))))))
  (Default|CallOnStatsUpdated (Variables|Default|GetCurrentHP) (Variables|Default|GetCurrentEP) (Variables|Default|GetIsDead) true))

(fn ShieldUp
  (params (InToMaximum :type Boolean) (InAddEP :type Integer))
  (if InToMaximum
    (Variables|Default|SetCurrentEP (.MaxEP (Utilities|Struct|BreakSTRUCT_MainStates (Variables|Default|GetMainStatsStructure))))
    (else
      (Variables|Default|SetCurrentEP (Math|Integer|Min(Integer) (+ InAddEP (Variables|Default|GetCurrentEP)) (.MaxEP (Utilities|Struct|BreakSTRUCT_MainStates (Variables|Default|GetMainStatsStructure)))))))
  (Default|CallOnStatsUpdated (Variables|Default|GetCurrentHP) (Variables|Default|GetCurrentEP) (Variables|Default|GetIsDead) true))

(fn CheckHP
  (return (== (Variables|Default|GetCurrentHP) (.MaxHP (Utilities|Struct|BreakSTRUCT_MainStates (Variables|Default|GetMainStatsStructure))))))

(fn CheckEp
  (return (== (Variables|Default|GetCurrentEP) (.MaxEP (Utilities|Struct|BreakSTRUCT_MainStates (Variables|Default|GetMainStatsStructure))))))

(fn ConfigureMovement
  (bind _mainstatsstructure (Variables|Default|GetMainStatsStructure))
  (bind _maxwalkspeed (Utilities|Struct|BreakSTRUCT_MainStates _mainstatsstructure))
  (if (Utilities|Enum|NotEqual(Enum) (.Type (Utilities|Struct|BreakSTRUCT_MainStates (Variables|Default|GetMainStatsStructure))) "NewEnumerator5")
    (bind _ascharacter (Utilities|Casting|CastToCharacter (Components|GetOwner)))
    (Variables|/Script/Engine.CharacterMovementComponent|SetMaxWalkSpeed (Variables|/Script/Engine.Character|GetCharacterMovement _ascharacter) _maxwalkspeed)
    (Variables|/Script/Engine.CharacterMovementComponent|SetMaxWalkSpeedCrouched (Variables|/Script/Engine.Character|GetCharacterMovement _ascharacter) (/ _maxwalkspeed 2.0))))

(fn ConfigureHealthandShields
  (bind _savegameobject (Utilities|CheckSaveGame)
    (:Is%20Valid
      (Variables|Default|SetCurrentHP (Variables|/Game/Blueprints/Object/BP_SaveGame.BP_SaveGame_C|GetSavedPlayerHP _savegameobject))
      (Variables|Default|SetCurrentEP (Variables|/Game/Blueprints/Object/BP_SaveGame.BP_SaveGame_C|GetSavedPlayerEP _savegameobject))
      (Default|CallOnStatsUpdated (Variables|Default|GetCurrentHP) (Variables|Default|GetCurrentEP) (Variables|Default|GetIsDead) false))
    (:False
      (CallFunction|HealUp true)
      (CallFunction|ShieldUp true))))

(fn UpdatedBehavior
  (params (InCurrentBehavior :type ENUM_Behavior%20Enum :default "NewEnumerator0"))
  (Variables|Default|SetCurrentBehavior InCurrentBehavior))

(fn UpdatedFraction
  (params (InCurrentFraction :type ENUM_Frations%20Enum :default "NewEnumerator0"))
  (Variables|Default|SetCurrentFraction InCurrentFraction))

(fn ConfigureBehaviorandFraction
  (CallFunction|UpdatedBehavior (Utilities|Struct|BreakSTRUCT_MainStates (Variables|Default|GetMainStatsStructure)))
  (CallFunction|UpdatedFraction (Utilities|Struct|BreakSTRUCT_MainStates (Variables|Default|GetMainStatsStructure))))