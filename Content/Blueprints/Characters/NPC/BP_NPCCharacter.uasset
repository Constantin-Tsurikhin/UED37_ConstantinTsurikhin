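; NPC character Blueprint with a health bar widget and support for AI patrol groups.
; On BeginPlay it binds the HP widget to itself.
; Setting a patrolling group above zero tells its BP_AiController to switch AI state, a call flagged with an error in the graph.
; ActionMain only forwards to the parent class.
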(event EventBeginPlay
  (|CallParentFunction)
  (bind _asw_heath_bar (Utilities|Casting|CastToW_HeathBar (UserInterface|GetUserWidgetObject (Variables|Default|GetWidgetHP))))
  (Default|UpdateCurrentCharacterforHP _asw_heath_bar self))

(event Collision|EventActorBeginOverlap
  (params (OtherActor :type Actor%20Object%20Reference))
  (|CallParentFunction OtherActor) ; This node is disabled and will not be called.\nDrag off pins to build functionality.
)

(event EventTick
  (params (DeltaSeconds :type Float%20%28single-precision%29))
  (|CallParentFunction DeltaSeconds) ; This node is disabled and will not be called.\nDrag off pins to build functionality.
)

(fn ConstructionScript
  (|CallParentFunction))

(fn ActionMain
  (params (IsPressed :type Boolean))
  (|CallParentFunction IsPressed))

(fn UpdatePatrollingGroup
  (params (InPatrollingGroup :type Byte))
  (Variables|Default|SetPatrollingGroup InPatrollingGroup)
  (if (> (Variables|Default|GetPatrollingGroup) 0)
    (bind _asbp_ai_controller (Utilities|Casting|CastToBP_AiController (AI|GetAIController self)))
    ;[1 1 1] Error
    (Default|UpdateAIState _asbp_ai_controller "NewEnumerator1")))