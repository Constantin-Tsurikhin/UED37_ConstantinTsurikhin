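; BP_Tumbler is an interactable toggle switch that switches the lock on a list of linked doors.
; Overlapping it shows a text prompt and enables Interact, which plays a timeline forward or in reverse to slide the stick mesh.
; When the timeline finishes, its direction sets the on/off state and each linked door's SwitchLock is called.
; The construction script positions the stick from the initial state.
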(event Custom|SwitchOn
  (if (not (Variables|Default|GetInProgress))
    (if (not (Variables|Default|GetIsTumblerON))
      (bind (_direction _move) (Timeline|TumblerTimeline PlayFromStart)
        (:Update
          (Variables|Default|SetInProgress false)
          (Transformation|SetRelativeLocation (Variables|Default|GetTumblerStickMesh) (Math|Vector|MakeVector 0.0 (* (Variables|Default|GetMaxStickOffset) _move) 0.0) false false))
        (:Finished
          (Variables|Default|SetInProgress false)
          (switch Utilities|FlowControl|Switch|SwitchonETimelineDirection _direction
            (:Forward
              (Variables|Default|SetIsTumblerON true))
            (:Backward
              (Variables|Default|SetIsTumblerON false)))
          (CallFunction|DoorsLockSwitch))))))

(event Custom|SwitchOff
  (if (not (Variables|Default|GetInProgress))
    (if (Variables|Default|GetIsTumblerON)
      (bind (_direction _move) (Timeline|TumblerTimeline ReverseFromEnd)
        (:Update
          (Variables|Default|SetInProgress false)
          (Transformation|SetRelativeLocation (Variables|Default|GetTumblerStickMesh) (Math|Vector|MakeVector 0.0 (* (Variables|Default|GetMaxStickOffset) _move) 0.0) false false))
        (:Finished
          (Variables|Default|SetInProgress false)
          (switch Utilities|FlowControl|Switch|SwitchonETimelineDirection _direction
            (:Forward
              (Variables|Default|SetIsTumblerON true))
            (:Backward
              (Variables|Default|SetIsTumblerON false)))
          (CallFunction|DoorsLockSwitch))))))

(event EventBeginPlay
  (Rendering|SetVisibility (Variables|Default|GetTextRender) false false))

(event Collision|EventActorBeginOverlap
  (params (OtherActor :type Actor%20Object%20Reference))
  (Rendering|SetVisibility (Variables|Default|GetTextRender) true false)
  (Variables|Default|SetIsReadyToInteract true))

(event EventTick
  (params (DeltaSeconds :type Float%20%28single-precision%29)))

(event Collision|EventActorEndOverlap
  (params (OtherActor :type Actor%20Object%20Reference))
  (Rendering|SetVisibility (Variables|Default|GetTextRender) false false)
  (Variables|Default|SetIsReadyToInteract false))

(fn ConstructionScript
  (Transformation|AddRelativeLocation (Variables|Default|GetTumblerStickMesh) (Math|Vector|MakeVector 0.0 (Math|Float|SelectFloat (Variables|Default|GetMaxStickOffset) 0.0 (Variables|Default|GetIsTumblerON)) 0.0) false false))

(fn DoorsLockSwitch
  (if (Utilities|Array|IsValidIndex (Variables|Default|GetDoorsToLockSwitch))
    (for _array_element (Variables|Default|GetDoorsToLockSwitch)
      (Default|SwitchLock _array_element))))

(fn Interact
  (if (Variables|Default|GetIsReadyToInteract)
    (if (Variables|Default|GetIsTumblerON)
      (CallFunction|SwitchOff)
      (return true)
      (else
        (CallFunction|Switchon)
        (return true)))
    (else
      (return false))))