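; BP_Trigger_NextLevel is a trigger that advances the game to the next level when the player reaches it.
; On overlap it runs the parent's overlap logic, then checks that the OverLappedActor variable is a BP_PlayerCharacter.
; It then calls UpdateNextLevel on BP_gameInstance, behind a DoOnce so the call fires only once per trigger instance.
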(event EventBeginPlay
  (|CallParentFunction) ; This node is disabled and will not be called.\nDrag off pins to build functionality.
)

(event Collision|EventActorBeginOverlap
  (params (OtherActor :type Actor%20Object%20Reference))
  (|CallParentFunction OtherActor)
  (Utilities|Casting|CastToBP_PlayerCharacter (Variables|Default|GetOverLappedActor))
  (bind _asbp_game_instance (Utilities|Casting|CastToBP_gameInstance (Game|GetGameInstance)))
  (Utilities|FlowControl|DoOnce false
    (:Completed
      (Default|UpdateNextLevel _asbp_game_instance))))

(event EventTick
  (params (DeltaSeconds :type Float%20%28single-precision%29))
  (|CallParentFunction DeltaSeconds) ; This node is disabled and will not be called.\nDrag off pins to build functionality.
)

(fn ConstructionScript
  (|CallParentFunction))