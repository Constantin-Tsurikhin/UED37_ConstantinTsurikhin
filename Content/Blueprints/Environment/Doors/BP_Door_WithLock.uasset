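; Lockable door Blueprint that extends a parent door class with a lock state and a colored indicator light.
; OpenDoor passes through to the parent only while the door is unlocked, while CloseDoor always passes through.
; SwitchLock toggles the lock, then refreshes the LockIndikator light to red when locked or green when unlocked.
; The Construction Script also refreshes the light, so it reflects the initial lock state.
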(event EventBeginPlay
  (|CallParentFunction) ; This node is disabled and will not be called.\nDrag off pins to build functionality.
)

(event Collision|EventActorBeginOverlap
  (params (OtherActor :type Actor%20Object%20Reference))
  (|CallParentFunction OtherActor) ; This node is disabled and will not be called.\nDrag off pins to build functionality.
)

(event EventTick
  (params (DeltaSeconds :type Float%20%28single-precision%29))
  (|CallParentFunction DeltaSeconds) ; This node is disabled and will not be called.\nDrag off pins to build functionality.
)

(event EventOpenDoor
  (if (not (Variables|DoorConfigure|GetIsLock))
    (|CallParentFunction)))

(event EventCloseDoor
  (|CallParentFunction))

(fn ConstructionScript
  (|CallParentFunction)
  (CallFunction|DoorLockIndication))

(fn SwitchLock
  (Variables|DoorConfigure|SetIsLock (not (Variables|DoorConfigure|GetIsLock)))
  (CallFunction|DoorLockIndication))

(fn DoorLockIndication
  (Rendering|Components|Light|SetLightColor (Variables|Default|GetLockIndikator) (Math|Color|SelectColor "(R=0.476042,G=0.000000,B=0.004551,A=1.000000)" "(R=0.220575,G=0.879167,B=0.000000,A=1.000000)" (Variables|DoorConfigure|GetIsLock)) true))