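; BP_AiHelper is a placeable AI helper marker that tracks overlapping characters and whether an NPC occupies it.
; Begin overlap records characters and clears Vacant for NPCs; end overlap is meant to reverse this, but its actor reference is None, so the cast fails.
; A Debug flag shows the arrow, mesh and sphere, and stores an overlapping player with a look-at-camera flag.
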(event EventBeginPlay
  (Rendering|SetVisibility (Variables|Default|GetArrow) (Variables|Default|GetDebug) false))

(event Collision|EventActorBeginOverlap
  (params (OtherActor :type Actor%20Object%20Reference))
  (Variables|Default|SetOtherActorBeginOverlap OtherActor)
  (Utilities|Casting|CastToBP_CharacterBase (Variables|Default|GetOtherActorBeginOverlap))
  (Utilities|Array|AddUnique (Variables|Default|GetOverlappedActors) (Variables|Default|GetOtherActorBeginOverlap))
  (Utilities|FlowControl|Sequence
    (:then_0
      (if (Variables|Default|GetDebug)
        (bind _asbp_player_character (Utilities|Casting|CastToBP_PlayerCharacter (Variables|Default|GetOtherActorBeginOverlap)))
        (Variables|Default|SetOverlappedPlayer _asbp_player_character)
        (Variables|Default|SetIsLookAtPlayerCamera true)))
    (:then_1
      (Utilities|Casting|CastToBP_NPCCharacter (Variables|Default|GetOtherActorBeginOverlap))
      (Variables|Default|SetVacant false))))

(event EventTick
  (params (DeltaSeconds :type Float%20%28single-precision%29)))

(event Collision|EventActorEndOverlap
  (params (OtherActor :type Actor%20Object%20Reference))
  (Variables|Default|SetOtherActorBeginOverlap 0)
  (Utilities|Casting|CastToBP_CharacterBase (Variables|Default|GetOtherActorBeginOverlap))
  (bind _returnvalue (Utilities|Array|RemoveItem (Variables|Default|GetOverlappedActors) (Variables|Default|GetOtherActorBeginOverlap)))
  (if _returnvalue
    (Utilities|FlowControl|Sequence
      (:then_0
        (if (Variables|Default|GetDebug)
          (bind _asbp_player_character (Utilities|Casting|CastToBP_PlayerCharacter (Variables|Default|GetOtherActorBeginOverlap)))
          (Variables|Default|SetOverlappedPlayer _asbp_player_character)
          (Variables|Default|SetIsLookAtPlayerCamera false)))
      (:then_1
        (Utilities|Casting|CastToBP_NPCCharacter (Variables|Default|GetOtherActorBeginOverlap))
        (if (Utilities|Array|IsValidIndex (Variables|Default|GetOverlappedActors))
          (Variables|Default|SetVacant false)
          (else
            (Variables|Default|SetVacant true)))))))

(fn ConstructionScript)