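; Sniper rifle ammo pickup that adds ammo to a character's backpack when interacted with.
; Overlapping shows a text prompt, caches the character and enables interaction; each tick the text rotates to face the player character's camera.
; Interact finds the character's BP_BackpackComponent, increases ammo by the item's name and amount, then destroys the pickup.
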(event EventBeginPlay
  (Rendering|SetVisibility (Variables|Default|GetTextRender) false false))

(event EventTick
  (params (DeltaSeconds :type Float%20%28single-precision%29))
  (CallFunction|LookingatPlayerCamera))

(event Collision|EventActorEndOverlap
  (params (OtherActor :type Actor%20Object%20Reference))
  (Rendering|SetVisibility (Variables|Default|GetTextRender) false false)
  (Variables|Default|SetIsReadyToInteract false)
  (Variables|Default|SetLookAt false)
  (Utilities|Casting|CastToCharacter OtherActor)
  (Variables|Default|SetCharacterInBox 0))

(event Collision|EventActorBeginOverlap
  (params (OtherActor :type Actor%20Object%20Reference))
  (Rendering|SetVisibility (Variables|Default|GetTextRender) true false)
  (Variables|Default|SetIsReadyToInteract true)
  (bind _ascharacter (Utilities|Casting|CastToCharacter OtherActor))
  (Variables|Default|SetCharacterInBox _ascharacter)
  (Variables|Default|GetCharacterInBox
    (:then
      (Variables|Default|SetLookAt true))
    (:else)))

(fn ConstructionScript)

(fn PutIntoBackpack
  (params (InBackpack :type BP%20Backpack%20Component%20Object%20Reference))
  (if (and (Utilities|Name|NotEqual(Name) (Variables|Default|GetItemName) "None") (> (Variables|Default|GetAmmo) 0))
    (Default|UpdateAmmobyName InBackpack (Variables|Default|GetItemName) (Variables|Default|GetAmmo) true)
    (CallFunction|AfterUse)))

(fn AfterUse
  (Actor|DestroyActor))

(fn LookingatPlayerCamera
  (if (Variables|Default|GetLookAt)
    (bind _characterinbox (Variables|Default|GetCharacterInBox)
      (:then
        (bind _asbp_player_character (Utilities|Casting|CastToBP_PlayerCharacter _characterinbox))
        (Variables|Default|SetCameraLOcation (Transformation|GetWorldLocation (Variables|/Game/Blueprints/Characters/Player/BP_PlayerCharacter.BP_PlayerCharacter_C|GetCamera _asbp_player_character)))
        (Transformation|SetWorldRotation (Variables|Default|GetTextRender) (Math|Rotator|FindLookatRotation (Transformation|GetWorldLocation (Variables|Default|GetTextRender)) (Variables|Default|GetCameraLOcation)) false false))
      (:else))))

(fn Interact
  (if (Variables|Default|GetIsReadyToInteract)
    (bind _characterinbox (Variables|Default|GetCharacterInBox)
      (:then
        (Utilities|IsValid (Actor|GetComponentbyClass _characterinbox "/Game/Components/BP_BackpackComponent.BP_BackpackComponent_C")
          (:Is%20Valid
            (CallFunction|PutIntoBackpack (Actor|GetComponentbyClass _characterinbox "/Game/Components/BP_BackpackComponent.BP_BackpackComponent_C"))
            (return true))
          (:Is%20Not%20Valid
            (return true))))
      (:else
        (return true)))
    (else
      (return true))))