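; Base item Blueprint for pickups that restore health, shield or both to a character instead of being stored in the backpack.
; Its PutIntoBackpack override skips the parent call and finds BP_MainStatsComponent on CharacterInBox, applying each positive restore value if the matching CheckHP or CheckEp returns false.
; AfterUse runs only if the item is flagged useful.
; HealUpToMaximum serves as the to-maximum input for both health and shield.
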(event EventBeginPlay
  (|CallParentFunction) ; This node is disabled and will not be called.\nDrag off pins to build functionality.
)

(event Collision|EventActorBeginOverlap
  (params (OtherActor :type Actor%20Object%20Reference))
  (|CallParentFunction OtherActor) ; This node is disabled and will not be called.\nDrag off pins to build functionality.
)

(event EventTick
  (params (DeltaSeconds :type Float%20%28single-precision%29))
  (|CallParentFunction DeltaSeconds) ; This node is disabled and will not be called.\nDrag off pins to build functionality.
)

(fn ConstructionScript
  (|CallParentFunction))

(fn PutIntoBackpack
  (params (InBackpack :type BP%20Backpack%20Component%20Object%20Reference))
  (bind _characterinbox (Variables|Default|GetCharacterInBox))
  (bind _returnvalue (Actor|GetComponentbyClass _characterinbox "/Game/Components/BP_MainStatsComponent.BP_MainStatsComponent_C"))
  (LocalVariables|SetL_BackPack InBackpack)
  (if (Utilities|Name|NotEqual(Name) (Variables|Default|GetItemName) "None")
    (Utilities|IsValid _returnvalue
      (:Is%20Valid
        (LocalVariables|SetL_MainStats _returnvalue)
        (Utilities|FlowControl|Sequence
          (:then_0
            (if (> (Variables|Default|GetHealUpValue) 0)
              (if (not (Default|CheckHP (LocalVariables|GetL_MainStats)))
                (Default|HealUp (LocalVariables|GetL_MainStats) (Variables|Default|GetHealUpToMaximum) (Variables|Default|GetHealUpValue))
                (Variables|Default|SetIsItUseful true))))
          (:then_1
            (if (> (Variables|Default|GetShieldUpValue) 0)
              (if (not (Default|CheckEp (LocalVariables|GetL_MainStats)))
                (Default|ShieldUp (LocalVariables|GetL_MainStats) (Variables|Default|GetHealUpToMaximum) (Variables|Default|GetShieldUpValue))
                (Variables|Default|SetIsItUseful true))))
          (:then_2
            (if (Variables|Default|GetIsItUseful)
              (CallFunction|AfterUse))))))))

(fn Interact
  (bind _success (|CallParentFunction))
  (return _success))