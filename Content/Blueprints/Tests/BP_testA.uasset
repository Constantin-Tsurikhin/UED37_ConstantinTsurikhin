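; BP_testA is a test actor that prints debug messages and shows a name on a text render component.
; On BeginPlay it calls a custom event twice, which prints a boolean parameter to screen in green or red.
; The construction script formats the Myname variable into the displayed text.
; A separate function forwards its name input to the same event, and Tick and overlap are empty.
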(event Custom|CustomEvent_0
  (params (NewParam :type Boolean) (NewParam2 :type Integer) (NewParam3 :type Byte) (NewParam4 :type Name))
  (Development|PrintString (Utilities|String|ToString(Boolean) NewParam) true false (Math|Color|SelectColor "(R=0.000000,G=1.000000,B=0.188644,A=1.000000)" "(R=1.000000,G=0.000000,B=0.010805,A=1.000000)" NewParam)))

(event EventBeginPlay
  (CallFunction|CustomEvent0 false 0 0 "None")
  (CallFunction|CustomEvent0 true 0 0 "None"))

(event Collision|EventActorBeginOverlap
  (params (OtherActor :type Actor%20Object%20Reference)))

(event EventTick
  (params (DeltaSeconds :type Float%20%28single-precision%29)))

(fn ConstructionScript
  (Rendering|Components|TextRender|SetText (Variables|Default|GetTextRender) (Utilities|Text|FormatText "My name is {Name}" (Variables|Test|GetMyname))))

(fn NewFunction0
  (params (InName :type Name) (InArray :type Array%20of%20Booleans))
  (CallFunction|CustomEvent0 false 0 0 InName))